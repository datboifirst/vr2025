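; Actor Blueprint that moves two cube components to target locations, one after the other.
; On BeginPlay it records the first cube's location, waits briefly, then plays a timeline that lerps that cube to its target.
; When that timeline finishes, it records the second cube's location and plays a second timeline that lerps it to its own target.
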(event `self.ReceiveBeginPlay`
  (set `self.SelfLocation` (`SceneComponent.K2_GetComponentLocation` (`self.Cube`)))
  (`KismetSystemLibrary.Delay` 2.0)
  (bind (_direction _time) (`Timeline|Timeline` :!via `PlayFromStart`)
    (:`Update`
      (`SceneComponent.K2_SetWorldLocation` (`self.Cube`) (`KismetMathLibrary.VLerp` (`self.SelfLocation`) (`self.TargetLocation`) _time) false false))
    (:`Finished`
      (set `self.SelfLocation_2` (`SceneComponent.K2_GetComponentLocation` (`self.Cube1`)))
      (bind (_direction_2 _time_2) (`Timeline|Timeline_0` :!via `PlayFromStart`)
        (:`Update`
          (`SceneComponent.K2_SetWorldLocation` (`self.Cube1`) (`KismetMathLibrary.VLerp` (`self.SelfLocation_2`) (`self.TargetLocation2`) _time_2) false false))))))

(fn `UserConstructionScript`)